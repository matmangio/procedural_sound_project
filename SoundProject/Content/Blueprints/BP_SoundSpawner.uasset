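; BP_SoundSpawner sets up the level's wind ambience on BeginPlay.
; It plays a non-spatialized large-obstacle wind MetaSound and spawns an attenuated tree-leaves MetaSound at every matching tree instance in the foliage actor.
; Trees are found by filtering the actor's hierarchical instanced mesh components against TreeMeshes.
; Each leaves sound receives its 2D distance from WindSource as the "Wind Distance" parameter, set once at spawn.
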(event EventBeginPlay
  (Utilities|FlowControl|Sequence
    (:then_0
      ;[0.8698 0.1911 0.5429 0.5] Spawn MSS_Wind_LargeObstacles, not spatialized
      (Audio|SpawnSound2D "/Game/Sounds/MSS_Wind_LargeObstacles.MSS_Wind_LargeObstacles" 0.25 1.0 0.0 0))
    (:then_1
      ;[0.245 0.8651 0.1546 0.5] Spawn MSS_Wind_TreeLeaves on each tree in the Foliage instance
      (for _array_element (Actor|GetComponentsByClass (Variables|Foliage|GetFoliageActor) "/Script/Engine.HierarchicalInstancedStaticMeshComponent")
        (if (Utilities|Array|ContainsItem (Variables|Foliage|GetTreeMeshes) (Variables|/Script/Engine.StaticMeshComponent|GetStaticMesh _array_element))
          (for _index (range 0 (- (Components|InstancedStaticMesh|GetInstanceCount _array_element) 1))
            (bind _returnvalue (Audio|SpawnSoundatLocation "/Game/Sounds/MSS_Wind_TreeLeaves.MSS_Wind_TreeLeaves" (.Location (Math|Transform|BreakTransform (.OutInstanceTransform (Components|InstancedStaticMesh|GetInstanceTransform _array_element _index true)))) "0, 0, 0" 0.4 1.0 0.0 "/Game/Sounds/Attenuation/SA_TreeLeaves.SA_TreeLeaves" 0))
            (Audio|Parameter|SetFloatParameter _returnvalue "Wind Distance" (Math|Vector|Distance2D(Vector) (.Location (Math|Transform|BreakTransform (.OutInstanceTransform (Components|InstancedStaticMesh|GetInstanceTransform _array_element _index true)))) (Transformation|GetActorLocation (Variables|Default|GetWind%20Source))) :!class /Script/AudioExtensions.AudioParameterControllerInterface) ; Set distance from wind source
          ))))))

(fn ConstructionScript)